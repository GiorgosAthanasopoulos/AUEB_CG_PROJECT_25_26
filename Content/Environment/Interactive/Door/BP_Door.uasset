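; Interactive door that swings open and closed when its Interact event passes an Activator equality check.
; ToggleDoor plays or reverses a timeline that lerps the Door component's relative location and rotation together.
; An animating flag blocks re-triggering mid-motion, and Pawn collision switches to Ignore as opening starts and back to Block as closing starts.
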(event `ToggleDoor`
  (if (`self.IsAnimating`)
    _
    (elif (`self.IsOpened`)
      (set `self.IsAnimating` true)
      (set `self.IsOpened` false)
      (`PrimitiveComponent.SetCollisionResponseToChannel` (`self.Door`) "ECC_Pawn" "ECR_Block")
      (bind (_direction _newtrack_0) (`Timeline|DoorOpen_Timeline` :!via `Reverse` :!label _label)
        (:`Update`
          (`SceneComponent.K2_SetRelativeLocationAndRotation` (`self.Door`) (`KismetMathLibrary.VLerp` (0.0 0.0 0.0) (-100.0 100.0 0.0) _newtrack_0) (`KismetMathLibrary.RLerp` (struct) (struct :`Yaw` 90.0) _newtrack_0) false false))
        (:`Finished`
          (set `self.IsAnimating` false)))
      (else
        (set `self.IsAnimating` true)
        (set `self.IsOpened` true)
        (`PrimitiveComponent.SetCollisionResponseToChannel` (`self.Door`) "ECC_Pawn" "ECR_Ignore")
        (goto _label)))))

(event `/Game/Environment/Interactive/BPI_Interactable.Interact`
  (params (Activator :type "Actor Object Reference"))
  (if (== Activator (`self.Activator`))
    (`self.ToggleDoor`)))

(fn `UserConstructionScript`)