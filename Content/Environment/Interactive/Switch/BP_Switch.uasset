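; BP_Switch is an interactive lever switch that triggers a referenced Interactable object when toggled.
; Its Interact event calls ToggleSwitch, which flips IsOpened and plays or reverses a timeline that lerps the Switch component's rotation between two angles.
; An IsAnimating flag blocks re-toggling mid-motion, and when the timeline finishes it clears the flag and calls Interact on the Interactable, passing itself.
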(event `ToggleSwitch`
  (if (`self.IsAnimating`)
    _
    (elif (`self.IsOpened`)
      (set `self.IsAnimating` true)
      (set `self.IsOpened` false)
      (bind (_direction _openalpha) (`Timeline|SwitchToggle_Timeline` :!via `Reverse` :!label _label)
        (:`Update`
          (`SceneComponent.K2_SetRelativeRotation` (`self.Switch`) (`KismetMathLibrary.RLerp` (struct :`Roll` -45.0) (struct :`Roll` -135.0) _openalpha) false false))
        (:`Finished`
          (set `self.IsAnimating` false)
          (`/Game/Environment/Interactive/BPI_Interactable.Interact` (`self.Interactable`) self)))
      (else
        (set `self.IsAnimating` true)
        (set `self.IsOpened` true)
        (goto _label)))))

(event `/Game/Environment/Interactive/BPI_Interactable.Interact`
  (params (Activator :type "Actor Object Reference"))
  (`self.ToggleSwitch`))

(fn `UserConstructionScript`)